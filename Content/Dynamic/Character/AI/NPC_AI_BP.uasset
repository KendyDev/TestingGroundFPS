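; AI controller Blueprint for a guard NPC that shoots at actors it perceives.
; On BeginPlay it sets up the PatrolData blackboard and runs the GuardBehaviour behavior tree.
; AI perception updates for actors without the "Enemy" tag toggle the controlled character's Aiming and Shooting flags with sensing success.
; The same updates set or clear the blackboard's enemy key.
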(event OnTargetPerceptionUpdated(AIPerception)
  (params (Actor :type Actor%20Object%20Reference) (Stimulus :type AI%20Stimulus%20Structure))
  (bind _bsuccessfullysensed (Utilities|Struct|BreakAIStimulus Stimulus))
  (bind _enemykey (Variables|Default|GetEnemyKey))
  (bind _blackboardcomp (Variables|Default|GetBlackboardComp))
  (if (not (Actor|ActorHasTag Actor "Enemy"))
    (bind _ascharacter (Utilities|Casting|CastToCharacter (Pawn|GetControlledPawn)))
    (bind _output_get (Variables|/Game/Dynamic/Character/Behaviour/Character.Character_C|SetAiming _ascharacter _bsuccessfullysensed))
    (Variables|/Game/Dynamic/Character/Behaviour/Character.Character_C|SetShooting _ascharacter _output_get)
    (if _bsuccessfullysensed
      (AI|Components|Blackboard|SetValueasObject _blackboardcomp _enemykey Actor)
      (else
        (AI|Components|Blackboard|ClearValue _blackboardcomp _enemykey)))))

(event EventBeginPlay
  (bind _blackboardcomponent (Class|AIController|UseBlackboard "/Game/Dynamic/Character/AI/PatrolData.PatrolData"))
  (AI|RunBehaviorTree "/Game/Dynamic/Character/AI/GuardBehaviour.GuardBehaviour")
  (Variables|Default|SetBlackboardComp _blackboardcomponent))

(fn ConstructionScript)