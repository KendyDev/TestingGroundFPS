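; AI controller for patrolling guard NPCs that runs their behavior tree and reacts to perceived targets.
; On BeginPlay it sets up the PatrolData blackboard and starts GuardBehaviour.
; Perception updates for actors without the "Enemy" tag set the guard pawn's Aiming and Shooting flags from whether sensing succeeded.
; The same update stores the actor as the blackboard enemy, or clears that key when sensing fails.
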(event OnTargetPerceptionUpdated(AIPerception)
  (params (Actor :type Actor%20Object%20Reference) (Stimulus :type AI%20Stimulus%20Structure))
  (bind _bsuccessfullysensed (Utilities|Struct|BreakAIStimulus Stimulus))
  (bind _enemykey (Variables|Default|GetEnemyKey))
  (bind _blackboardcomp (Variables|Default|GetBlackboardComp))
  (if (not (Actor|ActorHasTag Actor "Enemy"))
    (bind _asnew_patrolling_guard_bp (Utilities|Casting|CastToNew_PatrollingGuard_BP (Pawn|GetControlledPawn)))
    (bind _output_get (Variables|/Game/Dynamic/NPC/Behaviour/New_PatrollingGuard_BP.New_PatrollingGuard_BP_C|SetAiming _asnew_patrolling_guard_bp _bsuccessfullysensed))
    (Variables|/Game/Dynamic/NPC/Behaviour/New_PatrollingGuard_BP.New_PatrollingGuard_BP_C|SetShooting _asnew_patrolling_guard_bp _output_get)
    (if _bsuccessfullysensed
      (AI|Components|Blackboard|SetValueasObject _blackboardcomp _enemykey Actor)
      (else
        (AI|Components|Blackboard|ClearValue _blackboardcomp _enemykey)))))

(event EventBeginPlay
  (bind _blackboardcomponent (Class|AIController|UseBlackboard "/Game/Dynamic/NPC/AI/PatrolData.PatrolData"))
  (AI|RunBehaviorTree "/Game/Dynamic/NPC/AI/GuardBehaviour.GuardBehaviour")
  (Variables|Default|SetBlackboardComp _blackboardcomponent))

(fn ConstructionScript)